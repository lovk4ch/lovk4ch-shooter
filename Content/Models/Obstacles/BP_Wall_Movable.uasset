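; BP_Wall_Movable is an obstacle wall that slides back and forth along the world Y axis.
; Each tick, SetSpacing moves the Spacing value at a constant speed and flips IsReverse when the next step would pass either symmetric limit.
; The actor's Y is then set directly to Spacing, so the sweep is centered on world zero rather than the placed position, while X and Z stay unchanged.
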(event EventTick
  (params (DeltaSeconds :type Float%20%28single-precision%29))
  (bind _returnvalue (Transformation|GetActorLocation))
  (CallFunction|SetSpacing DeltaSeconds)
  (Transformation|SetActorLocation (Math|Vector|MakeVector (.x _returnvalue) (Variables|Params|GetSpacing) (.z _returnvalue)) false false))

(fn ConstructionScript
  (|CallParentFunction))

(fn SetSpacing
  (params (Delta :type Float%20%28single-precision%29))
  (bind _returnvalue (* Delta 4e+02))
  (if (Variables|Params|GetisReverse)
    (if (> (+ (Variables|Params|GetSpacing) _returnvalue) 1.75e+03)
      (Variables|Params|SetisReverse (not (Variables|Params|GetisReverse)))
      (else
        (Variables|Params|SetSpacing (+ (Variables|Params|GetSpacing) _returnvalue))))
    (elif (< (- (Variables|Params|GetSpacing) _returnvalue) -1.75e+03)
      (Variables|Params|SetisReverse (not (Variables|Params|GetisReverse)))
      (else
        (Variables|Params|SetSpacing (- (Variables|Params|GetSpacing) _returnvalue))))))