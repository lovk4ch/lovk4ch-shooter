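; Vehicle actor Blueprint for the Cyber machine, with an armor pool that damage depletes until the actor is destroyed.
; BeginPlay caches the WBP_Machine_HealthBar from its widget component, and Tick pushes the armor fraction to it every frame.
; Any damage is subtracted from Armor through CheckForProjectile, which applies no projectile check and destroys the actor at zero or below.
; A CheckCollision function destroys it unconditionally, but nothing in this file calls it.
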(event Game|Damage|EventAnyDamage
  (params (Damage :type Float%20%28single-precision%29) (DamageType :type Damage%20Type%20Object%20Reference) (InstigatedBy :type Controller%20Object%20Reference) (DamageCauser :type Actor%20Object%20Reference))
  (CallFunction|CheckforProjectile Damage))

(event EventBeginPlay
  (bind _aswbp_machine_health_bar (Utilities|Casting|CastToWBP_Machine_HealthBar (UserInterface|GetUserWidgetObject (Variables|Default|GetHealthBar))))
  (Variables|References|SetHealthBarWidget _aswbp_machine_health_bar))

(event EventTick
  (params (DeltaSeconds :type Float%20%28single-precision%29))
  (Variables|/Game/Widgets/WBP_Machine_HealthBar.WBP_Machine_HealthBar_C|SetArmor (Variables|References|GetHealthBarWidget) (/ (Variables|Params|GetArmor) (Variables|Params|GetMaxArmor))))

(fn ConstructionScript)

(fn Destroy
  (Actor|DestroyActor))

(fn CheckCollision
  (params (Other%20Actor :type Actor%20Object%20Reference))
  (CallFunction|Destroy))

(fn CheckforProjectile
  (params (Damage :type Float%20%28single-precision%29))
  (Variables|Params|SetArmor (- (Variables|Params|GetArmor) Damage))
  (if (<= (Variables|Params|GetArmor) 0.0)
    (CallFunction|Destroy)))