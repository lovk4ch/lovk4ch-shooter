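; Player-controlled cyber vehicle Blueprint that moves sideways along Y and fires projectiles.
; Move axis input offsets the actor by MoveSpeed, snapping it to the Bounds edge when it would go past.
; Holding Fire runs a self-re-entering Gate and Delay loop that spawns BP_Projectile from the Gun every ShootInterval until release.
; Overlaps call the CheckCollision override, which only casts to BP_Machine_Cyber_Enemy, leaving the parent call unconnected.
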(event Collision|EventActorBeginOverlap
  (params (OtherActor :type Actor%20Object%20Reference))
  ;[1 1 1] Collision logic
  (CallFunction|CheckCollision OtherActor))

(event Input|ActionEvents|InputActionFire
  (params (Key :type Key%20Structure :default "None"))
  ;[1 1 1] Fire logic
  (:Pressed
    (Utilities|FlowControl|Sequence
      (:then_0
        (goto _label Open))
      (:then_1
        (Utilities|FlowControl|Gate true :!label _label
          (:Exit
            (Game|SpawnActorfromClass "/Game/Models/Projectiles/BP_Projectile.BP_Projectile_C" (Transformation|GetWorldTransform (Variables|Default|GetGun)) "Undefined" self "NewEnumerator1" 0)
            (Utilities|FlowControl|Delay (Variables|Default|GetShoot%20Interval))
            (goto _label))))))
  (:Released
    (goto _label Close)))

(event Input|AxisEvents|InputAxisMove
  (params (AxisValue :type Float%20%28single-precision%29))
  (bind _returnvalue (Transformation|GetActorLocation))
  (bind _move_speed (Variables|Default|GetMove%20Speed))
  (bind _returnvalue_2 (* AxisValue _move_speed))
  ;[1 1 1] Player movement
  (if (< (Math|Float|Absolute(Float) (+ (.y (Transformation|GetActorLocation)) _returnvalue_2)) (Variables|Default|GetBounds))
    (Transformation|AddActorLocalOffset (Math|Vector|MakeVector 0.0 _returnvalue_2 0.0) false false)
    (else
      (Transformation|SetActorLocation (Math|Vector|MakeVector (.x _returnvalue) (* (Variables|Default|GetBounds) (Math|Float|Sign(Float) (.y _returnvalue))) (.z _returnvalue)) false false))))

(fn ConstructionScript
  (|CallParentFunction))

(fn CheckCollision
  (params (Other%20Actor :type Actor%20Object%20Reference))
  (Utilities|Casting|CastToBP_Machine_Cyber_Enemy Other%20Actor))