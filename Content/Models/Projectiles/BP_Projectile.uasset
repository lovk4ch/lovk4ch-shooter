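; BP_Projectile is a moving projectile actor that damages enemy or player Cyber machines.
; On overlap, its Enemy setting selects which machine subclass receives Damage before it self-destructs; other machines leave it intact, while non-machine actors destroy it.
; Tick moves it without sweeping, passing the world forward vector scaled by Speed as a local offset.
; A short lifespan set at BeginPlay removes stray shots.
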(event OnComponentBeginOverlap(Projectile)
  (params (OverlappedComponent :type Primitive%20Component%20Object%20Reference) (OtherActor :type Actor%20Object%20Reference) (OtherComp :type Primitive%20Component%20Object%20Reference) (OtherBodyIndex :type Integer) (bFromSweep :type Boolean) (SweepResult :type Hit%20Result%20Structure%20%28by%20ref%29))
  (bind _asbp_machine_cyber (Utilities|Casting|CastToBP_Machine_Cyber OtherActor)
    (:then
      (switch Utilities|FlowControl|Switch|SwitchonE_ProjectileOwnerType "NewEnumerator0"
        (:NewEnumerator0
          (bind _asbp_machine_cyber_enemy (Utilities|Casting|CastToBP_Machine_Cyber_Enemy _asbp_machine_cyber))
          (Game|Damage|ApplyDamage _asbp_machine_cyber_enemy (Variables|Params|GetDamage) 0 0))
        (:NewEnumerator1
          (bind _asbp_machine_cyber_player (Utilities|Casting|CastToBP_Machine_Cyber_Player _asbp_machine_cyber))
          (Game|Damage|ApplyDamage _asbp_machine_cyber_player (Variables|Params|GetDamage) 0 0)))
      (Actor|DestroyActor))
    (:CastFailed
      (Actor|DestroyActor))))

(event EventBeginPlay
  (Actor|SetLifeSpan 3.0))

(event EventTick
  (params (DeltaSeconds :type Float%20%28single-precision%29))
  (Transformation|AddActorLocalOffset (* (Transformation|GetActorForwardVector) (* DeltaSeconds (Variables|Params|GetSpeed))) false false))

(fn ConstructionScript)