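; BP_Machine_Cyber_Player is the player-controlled shooter, which slides sideways along Y and fires projectiles.
; The Move axis offsets it by MoveSpeed, snapping it to the Bounds limit on its current side when a step would overshoot.
; Fire spawns a BP_Projectile at the Gun transform, flagged as non-enemy.
; Overlapping enemy projectiles are destroyed, with no damage applied to the player here.
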(event Collision|EventActorBeginOverlap
  (params (OtherActor :type Actor%20Object%20Reference))
  (bind _asbp_projectile (Utilities|Casting|CastToBP_Projectile OtherActor))
  (if (Variables|/Game/Models/BP_Projectile.BP_Projectile_C|GetisEnemyProjectile _asbp_projectile)
    (Actor|DestroyActor _asbp_projectile)))

(event Input|ActionEvents|InputActionFire
  (params (Key :type Key%20Structure :default "None"))
  (:Pressed
    (bind _returnvalue (Game|SpawnActorfromClass "/Game/Models/BP_Projectile.BP_Projectile_C" (Transformation|GetWorldTransform (Variables|Default|GetGun)) "Undefined" 0 0))
    (Variables|/Game/Models/BP_Projectile.BP_Projectile_C|SetisEnemyProjectile _returnvalue false)))

(event Input|AxisEvents|InputAxisMove
  (params (AxisValue :type Float%20%28single-precision%29))
  (bind _returnvalue (Transformation|GetActorLocation))
  (bind _move_speed (Variables|Default|GetMove%20Speed))
  (bind _returnvalue_2 (* AxisValue _move_speed))
  ;[1 1 1] Player movement
  (if (< (Math|Float|Absolute(Float) (+ (.y (Transformation|GetActorLocation)) _returnvalue_2)) (Variables|Default|GetBounds))
    (Transformation|AddActorLocalOffset (Math|Vector|MakeVector 0.0 _returnvalue_2 0.0) false false)
    (else
      (Transformation|SetActorLocation (Math|Vector|MakeVector (.x _returnvalue) (* (Variables|Default|GetBounds) (Math|Float|Sign(Float) (.y _returnvalue))) (.z _returnvalue)) false false))))

(fn ConstructionScript
  (|CallParentFunction))