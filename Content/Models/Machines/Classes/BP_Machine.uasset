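; BP_Machine is an actor for combat machines with armor, a health bar and projectile shooting, crediting player machines for kills.
; Shoot spawns a BP_Projectile at the given gun's transform, tagged with the owner type, and returns the shoot interval.
; Damage reduces armor; at zero the machine calls AddScore on a BP_Machine_Player damage causer and destroys itself.
; Tick feeds the armor ratio to the widget, and CheckCollision destroys the machine outright.
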(event Game|Damage|EventAnyDamage
  (params (Damage :type Float%20%28single-precision%29) (DamageType :type Damage%20Type%20Object%20Reference) (InstigatedBy :type Controller%20Object%20Reference) (DamageCauser :type Actor%20Object%20Reference))
  (CallFunction|SetArmor Damage DamageCauser))

(event EventBeginPlay
  (bind _aswbp_machine_health_bar (Utilities|Casting|CastToWBP_Machine_HealthBar (UserInterface|GetUserWidgetObject (Variables|Default|GetHealthBar))))
  (Variables|References|SetHealthBarWidget _aswbp_machine_health_bar))

(event EventTick
  (params (DeltaSeconds :type Float%20%28single-precision%29))
  (Variables|/Game/Widgets/WBP_Machine_HealthBar.WBP_Machine_HealthBar_C|SetArmor (Variables|References|GetHealthBarWidget) (/ (Variables|Params|GetArmor) (Variables|Params|GetMaxArmor))))

(fn ConstructionScript)

(fn Shoot
  (params (Gun :type Scene%20Component%20Object%20Reference) (OwnerType :type E_ProjectileOwnerType%20Enum :default "NewEnumerator0"))
  (Game|SpawnActorfromClass "/Game/Models/Projectiles/BP_Projectile.BP_Projectile_C" (Transformation|GetWorldTransform Gun) "Undefined" self OwnerType 0)
  (return (Variables|Params|GetShoot%20Interval)))

(fn Destroy
  (Actor|DestroyActor))

(fn CheckCollision
  (params (Other%20Actor :type Actor%20Object%20Reference))
  (CallFunction|Destroy))

(fn SetArmor
  (params (Damage :type Float%20%28single-precision%29) (Owner :type Actor%20Object%20Reference))
  (Variables|Params|SetArmor (- (Variables|Params|GetArmor) Damage))
  (if (<= (Variables|Params|GetArmor) 0.0)
    (bind _asbp_machine_player (Utilities|Casting|CastToBP_Machine_Player Owner)
      (:then
        (Default|AddScore _asbp_machine_player))
      (:CastFailed
        _))
    (CallFunction|Destroy)))