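; Enemy machine Blueprint that creeps along negative X, with an externally set Y offset applied around its spawn position.
; Attack line-traces forward and, unless another enemy is hit, either shoots or occasionally sets IsHit, which freezes the offset and turns the creep into a fast charge.
; Overlaps with walls or the player machine run parent collision handling, and Destroy removes the enemy from GameMode_Game.
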(event Custom|SetDelta
  (params (Delta :type Float%20%28single-precision%29))
  ;[1 1 1] Move logic
  (if (not (Variables|Params|GetisHit))
    (Variables|Params|SetDelta Delta)))

(event EventTick
  (params (DeltaSeconds :type Float%20%28single-precision%29))
  ;[1 1 1] Move logic
  (|CallParentFunction DeltaSeconds)
  (CallFunction|SetPosition)
  (Transformation|SetActorLocation (Math|Vector|MakeVector (Variables|Params|GetPositionX) (+ (Variables|Params|GetPositionY) (Variables|Params|GetDelta)) (.z (Transformation|GetActorLocation))) false false))

(event Collision|EventActorBeginOverlap
  (params (OtherActor :type Actor%20Object%20Reference))
  (CallFunction|CheckCollision OtherActor))

(event EventBeginPlay
  (bind _returnvalue (Transformation|GetActorLocation))
  (|CallParentFunction)
  (Variables|Params|SetPositionX (.x _returnvalue))
  (Variables|Params|SetPositionY (.y _returnvalue)))

(fn ConstructionScript
  (|CallParentFunction))

(fn SetPosition
  (if (Variables|Params|GetisHit)
    (Variables|Params|SetPositionX (- (Variables|Params|GetPositionX) (* (Utilities|Time|GetWorldDeltaSeconds) 9e+02)))
    (else
      (Variables|Params|SetPositionX (- (Variables|Params|GetPositionX) (* (Utilities|Time|GetWorldDeltaSeconds) 3e+01))))))

(fn Destroy
  (bind _asgame_mode_game (Utilities|Casting|CastToGameMode_Game (Game|GetGameMode)))
  (Default|RemoveEnemy _asgame_mode_game self)
  (|CallParentFunction))

(fn Shoot
  (params (Gun :type Scene%20Component%20Object%20Reference) (OwnerType :type E_ProjectileOwnerType%20Enum :default "NewEnumerator0"))
  (bind _delay (|CallParentFunction Gun "NewEnumerator0"))
  (return _delay))

(fn Attack
  (bind _rootcomponent (Variables|Transformation|GetRootComponent))
  (bind _returnvalue (Math|Vector|GetUpVector _rootcomponent))
  (bind _returnvalue_2 (Transformation|GetWorldLocation _rootcomponent))
  (bind _returnvalue_3 (* _returnvalue 4e+01))
  (bind _returnvalue_4 (+ _returnvalue_2 _returnvalue_3))
  (bind _outhit (Collision|LineTraceByChannel _returnvalue_4 (+ _returnvalue_4 (* (Math|Vector|GetForwardVector _rootcomponent) 4e+03)) "TraceTypeQuery1" false 0 "ForDuration"))
  (Utilities|Casting|CastToBP_Machine_Enemy (.hitactor _outhit)
    (:CastFailed
      (if (> (Math|Random|RandomIntegerinRange 0 15) 14)
        (Variables|Params|SetisHit true)
        (else
          (CallFunction|Shoot 0 "NewEnumerator0"))))))

(fn CheckCollision
  (params (Other%20Actor :type Actor%20Object%20Reference))
  (Utilities|FlowControl|Sequence
    (:then_0
      (Utilities|Casting|CastToBP_Wall Other%20Actor))
    (:then_1
      (Utilities|Casting|CastToBP_Machine_Player Other%20Actor)))
  (|CallParentFunction 0))